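; TheGameManager is a game-state manager for a side-scroller that switches the UI to match the current state.
; Init has the SideScrollerGameMode create the UI.
; SetState ignores repeated states, otherwise hides the UI and stores the new state; only Running has further handling, hiding the mouse and showing the health widget through ShowHUD.
; Its event graph holds only disabled placeholder events, so other code must drive it.
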(fn `GetState`
  (returns (GameState :type "/Game/NathansContent/Blueprints/GameStates Enum"))
  (return (`self.Current Game State`)))

(fn `Init`
  (bind _asside_scroller_game_mode (cast `/Game/SideScrollerBP/Blueprints/SideScrollerGameMode` (`GameplayStatics.GetGameMode`)))
  (`/Game/SideScrollerBP/Blueprints/SideScrollerGameMode.CreateUI` _asside_scroller_game_mode))

(fn `SetState`
  (params (`New State` :type "/Game/NathansContent/Blueprints/GameStates Enum" :default "NewEnumerator0"))
  (if (!= `New State` (`self.Current Game State`))
    (`/Game/NathansContent/Blueprints/NathansFunctionLibrary.HideUI`)
    (bind _output_get (set `self.Current Game State` `New State`))
    (switch `/Game/NathansContent/Blueprints/GameStates` _output_get
      (:`NewEnumerator0`
        (`/Game/NathansContent/Blueprints/NathansFunctionLibrary.ShowMouse` false)
        (`self.ShowHUD` true)))))

(fn `ShowHUD`
  (params (Visible :type Boolean))
  (bind _widget_health (`self.Widget_health`))
  (if Visible
    (`Widget.SetVisibility` _widget_health "Visible")
    (else
      (`Widget.SetVisibility` _widget_health "Hidden"))))

(fn `UserConstructionScript`)